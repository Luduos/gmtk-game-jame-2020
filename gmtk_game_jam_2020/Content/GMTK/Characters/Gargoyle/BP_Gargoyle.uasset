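; BP_Gargoyle is a flying hazard that homes in on the player pawn through its ProjectileMovement component.
; Overlapping the player with DamageCollider applies environment damage once.
; Paddle damage turns off the collider's overlaps, making it harmless, and schedules delayed destruction.
; A dot product check on Tick stops homing once it falls behind the target's forward direction, then also schedules destruction.
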(event OnComponentBeginOverlap(DamageCollider)
  (params (OverlappedComponent :type Primitive%20Component%20Object%20Reference) (OtherActor :type Actor%20Object%20Reference) (OtherComp :type Primitive%20Component%20Object%20Reference) (OtherBodyIndex :type Integer) (bFromSweep :type Boolean) (SweepResult :type Hit%20Result%20Structure%20%28by%20ref%29))
  ;[1 1 1] Only apply damage to player once
  (bind _aspawn (Utilities|Casting|CastToPawn OtherActor))
  (if (Pawn|IsPlayerControlled _aspawn)
    (Utilities|FlowControl|DoOnce false
      (:Completed
        (Game|Damage|ApplyDamage _aspawn (Variables|Config|GetDamage) 0 self "/Game/GMTK/Environment/Damaging/BP_EnvironmentDamageType.BP_EnvironmentDamageType_C")))))

(event Game|Damage|EventAnyDamage
  (params (Damage :type Float%20%28single-precision%29) (DamageType :type Damage%20Type%20Object%20Reference) (InstigatedBy :type Controller%20Object%20Reference) (DamageCauser :type Actor%20Object%20Reference))
  (Utilities|Casting|CastToBP_PaddleDamageType DamageType)
  ;[1 1 1] if hit, don't damage player anymore
  (Variables|/Script/Engine.PrimitiveComponent|SetbGenerateOverlapEvents (Variables|Default|GetDamageCollider) false)
  (Utilities|DelayedDestruction 5.0))

(event EventTick
  (params (DeltaSeconds :type Float%20%28single-precision%29))
  (bind _projectilemovement (Variables|Default|GetProjectileMovement))
  (bind _homingtargetcomponent (Variables|/Script/Engine.ProjectileMovementComponent|GetHomingTargetComponent _projectilemovement))
  ;[1 1 1] if we're behind the target
  (Utilities|IsValid _homingtargetcomponent
    (:Is%20Valid
      (if (< (Math|Vector|DotProduct (- (Transformation|GetActorLocation) (Transformation|GetWorldLocation _homingtargetcomponent)) (Math|Vector|GetForwardVector _homingtargetcomponent)) 0.0)
        ;[1 1 1] Stop following
        (Variables|/Script/Engine.ProjectileMovementComponent|SetbIsHomingProjectile (Variables|Default|GetProjectileMovement) false)
        (Utilities|DelayedDestruction 5.0)))))

(event EventBeginPlay
  (bind _returnvalue (Game|Player|GetPlayerPawn 0))
  (Utilities|IsValid _returnvalue
    (:Is%20Valid
      (Variables|/Script/Engine.ProjectileMovementComponent|SetHomingTargetComponent (Variables|Default|GetProjectileMovement) (Variables|/Script/Engine.Actor|GetRootComponent _returnvalue)))))

(fn ConstructionScript)