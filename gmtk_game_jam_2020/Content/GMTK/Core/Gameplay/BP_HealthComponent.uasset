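; BP_HealthComponent is a health component that tracks current healthpoints, starting at the maximum on BeginPlay.
; Damage and healing events subtract from or add to the current value through a shared UpdateHealth function.
; UpdateHealth stores the value without clamping, fires OnDeath at zero or below, then always broadcasts OnHealthChanged.
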(event Custom|OnReceiveDamage
  (params (Damage :type Float%20%28single-precision%29))
  (CallFunction|UpdateHealth (- (Variables|Default|GetCurrentHealthpoints) Damage)))

(event Custom|OnReceiveHealing
  (params (Healing :type Float%20%28single-precision%29))
  (CallFunction|UpdateHealth (+ (Variables|Default|GetCurrentHealthpoints) Healing)))

(event EventBeginPlay
  (CallFunction|UpdateHealth (Variables|Config|GetMaxHealthpoints)))

(fn UpdateHealth
  (params (NewHealth :type Float%20%28single-precision%29))
  (bind _output_get (Variables|Default|SetCurrentHealthpoints NewHealth))
  (if (<= _output_get 0.0)
    (Default|CallOnDeath))
  (Default|CallOnHealthChanged (Variables|Default|GetCurrentHealthpoints)))