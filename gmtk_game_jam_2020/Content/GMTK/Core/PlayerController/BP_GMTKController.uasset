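; BP_GMTKController is a player controller that turns axis inputs into movement and look for whichever pawn it controls.
; MoveForward, MoveRight and MoveUp add movement input along axes built from control yaw only, so movement ignores camera pitch and pawn mesh rotation.
; Turn and LookUp feed controller yaw and pitch through the pawn.
; Every input first passes the GetControlledPawnValid macro, acting only when a pawn is valid.
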(event Input|AxisEvents|InputAxisMoveUp
  (params (AxisValue :type Float%20%28single-precision%29))
  ;[1 1 1] Player Input Movement
  (bind _controlled_pawn (Utilities|GetControlledPawnValid)
    (:Valid
      (Pawn|Input|AddMovementInput _controlled_pawn (Math|Vector|GetUpVector (Math|Rotator|MakeRotator 0.0 0.0 (.yaw (Pawn|GetControlRotation :!class /Script/Engine.Controller)))) AxisValue false))))

(event Input|AxisEvents|InputAxisMoveForward
  (params (AxisValue :type Float%20%28single-precision%29))
  ;[1 1 1] Player Input Movement
  (bind _controlled_pawn (Utilities|GetControlledPawnValid)
    (:Valid
      (Pawn|Input|AddMovementInput _controlled_pawn (Math|Vector|GetForwardVector (Math|Rotator|MakeRotator 0.0 0.0 (.yaw (Pawn|GetControlRotation :!class /Script/Engine.Controller)))) AxisValue false))))

(event Input|AxisEvents|InputAxisMoveRight
  (params (AxisValue :type Float%20%28single-precision%29))
  ;[1 1 1] Player Input Movement
  (bind _controlled_pawn (Utilities|GetControlledPawnValid)
    (:Valid
      (Pawn|Input|AddMovementInput _controlled_pawn (Math|Vector|GetRightVector (Math|Rotator|MakeRotator 0.0 0.0 (.yaw (Pawn|GetControlRotation :!class /Script/Engine.Controller)))) AxisValue false))))

(event Input|AxisEvents|InputAxisLookUp
  (params (AxisValue :type Float%20%28single-precision%29))
  ;[1 1 1] Look Up Down
  (bind _controlled_pawn (Utilities|GetControlledPawnValid)
    (:Valid
      (Pawn|Input|AddControllerPitchInput _controlled_pawn AxisValue))))

(event Input|AxisEvents|InputAxisTurn
  (params (AxisValue :type Float%20%28single-precision%29))
  ;[1 1 1] Turn
  (bind _controlled_pawn (Utilities|GetControlledPawnValid)
    (:Valid
      (Pawn|Input|AddControllerYawInput _controlled_pawn AxisValue))))

(fn ConstructionScript)