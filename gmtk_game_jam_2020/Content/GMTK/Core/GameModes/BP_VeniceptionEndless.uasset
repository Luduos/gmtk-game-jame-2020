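; Endless game mode for Veniception that sets up the boat player and keeps spawning track pieces as the game progresses.
; On BeginPlay it links the player to the map's BP_Boat, binds a debug-print death handler and picks a starting turnable by forward-projected location.
; Each turnable's spawn-next event spawns a random type at an offset, moves it to the target and binds its event, chaining indefinitely while counting spawned fields.
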(event Custom|OnPlayerDeath
  (Development|PrintString "WE DEAD"))

(event Custom|OnSpawnNext_Event
  (params (SpawnNextTarget :type Transform))
  (bind _newparam (CallFunction|SpawnNext SpawnNextTarget))
  (EventDispatchers|BindEventtoOnSpawnNextEntered _newparam (delegate Custom|OnSpawnNext_Event))
  (Math|Integer|IncrementInt (Variables|Default|GetSpawnedFields)))

(event EventBeginPlay
  ;[1 1 1] Get boat
  (bind _returnvalue (Actor|GetActorOfClass "/Game/GMTK/Interactables/Boat/BP_Boat.BP_Boat_C"))
  (Utilities|IsValid _returnvalue
    (:Is%20Valid
      (Variables|Default|SetBoat _returnvalue)
      ;[1 1 1] Set Player to boat
      (bind _asbp_boat_character (Utilities|Casting|CastToBP_BoatCharacter (Game|GetPlayerCharacter 0)))
      (bind _output_get (Variables|Default|SetPlayer _asbp_boat_character))
      (Default|SetBoatPlayerPosition _output_get (Default|GetPlayerPositionComponent (Variables|Default|GetBoat)))
      ;[1 1 1] Bind Player Death event
      (EventDispatchers|BindEventtoPlayerDeath (Variables|Default|GetPlayer) (delegate Custom|OnPlayerDeath))
      (bind _newparam (CallFunction|FindFurthestTurnable))
      (EventDispatchers|BindEventtoOnSpawnNextEntered _newparam (delegate Custom|OnSpawnNext_Event)))
    (:Is%20Not%20Valid
      (Development|PrintString "Couldn't find boat, please add a BP_Boat to the map"))))

(fn ConstructionScript)

(fn FindFurthestTurnable
  (bind _outactors (Actor|GetAllActorsOfClass "/Game/GMTK/Environment/Turning/BP_TurnableMaster.BP_TurnableMaster_C"))
  (for _array_element _outactors
    (if (> (Math|Vector|DotProduct (Transformation|GetActorForwardVector _array_element) (Transformation|GetActorLocation _array_element)) (LocalVariables|GetMaxForwardValue))
      (LocalVariables|SetFurthestTurnable _array_element)))
  (return (LocalVariables|GetFurthestTurnable)))

(fn SpawnNext
  (params (SpawnTransform :type Transform))
  (bind _spawningdata (Variables|Config|GetSpawningData))
  (bind _turningspawntypes (Variables|/Game/GMTK/Environment/Turning/BP_TurningSpawnTypes.BP_TurningSpawnTypes_C|GetTurningSpawnTypes _spawningdata))
  (LocalVariables|SetSpawn%20Transform SpawnTransform)
  (bind _returnvalue (Game|SpawnActorfromClass (Utilities|Array|Get(acopy) _turningspawntypes (Math|Random|RandomInteger (Utilities|Array|Length _turningspawntypes))) (Math|Transform|MakeTransform (+ (Variables|/Game/GMTK/Environment/Turning/BP_TurningSpawnTypes.BP_TurningSpawnTypes_C|GetLocalSpawnDistance (Variables|Config|GetSpawningData)) (.location (LocalVariables|GetSpawn%20Transform))) (.rotation (LocalVariables|GetSpawn%20Transform)) (.scale (LocalVariables|GetSpawn%20Transform))) "Undefined" 0 0))
  (Default|MovetoTarget _returnvalue (LocalVariables|GetSpawn%20Transform))
  (return _returnvalue))