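; BP_Boat is a boat pawn that constantly moves forward, takes left/right steering input and exposes a player position component.
; Without sideways input, it nudges itself back toward its starting lateral line through FloatingPawnMovement.
; Each tick it adds a sine offset to the mesh height for bobbing and sets mesh pitch and roll for swaying.
; A downward trace stores the water position, which nothing here reads.
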(event Custom|OnLeftRightMovement
  (params (AxisValue :type Float%20%28single-precision%29))
  ;[1 1 1] Left Right movement
  (Class|PawnMovementComponent|AddInputVector (Variables|Default|GetFloatingPawnMovement) (* (Transformation|GetActorRightVector) AxisValue) true))

(event EventTick
  (params (DeltaSeconds :type Float%20%28single-precision%29))
  (bind _returnvalue (Transformation|GetActorLocation))
  (bind _returnvalue_2 (Transformation|GetActorRightVector))
  (bind _initiallocation (Variables|Default|GetInitialLocation))
  (bind _returnvalue_3 (- _initiallocation _returnvalue))
  (bind _returnvalue_4 (Math|Vector|DotProduct _returnvalue_2 _returnvalue_3))
  (Animation|UpdateWaterPositition)
  (Animation|UpdateBoatLocation DeltaSeconds)
  ;[1 1 1] Update Boat swaying
  (Transformation|SetRelativeRotation (Variables|Default|GetStaticMesh) (Math|Rotator|MakeRotator (Utilities|CalcPitch) (Utilities|CalcRoll) (.yaw (Variables|Animation|Swaying|GetInitalMeshRotation))) false false)
  ;[1 1 1] If there is no sideways input by the player
  (if (< (Math|Float|Absolute(Float) (Math|Vector|DotProduct (Transformation|GetActorRightVector) (Pawn|Components|PawnMovement|GetLastInputVector (Variables|Default|GetFloatingPawnMovement)))) 0.01)
    ;[1 1 1] if we're far enough away from the center
    (if (> (Math|Float|Absolute(Float) _returnvalue_4) 1e+01)
      ;[1 1 1] Add input to move back to center
      (Class|PawnMovementComponent|AddInputVector (Variables|Default|GetFloatingPawnMovement) (* (* (Transformation|GetActorRightVector) (Math|Float|Sign(Float) _returnvalue_4)) (Variables|Config|GetBackToCenterForceMultiplicator)) false))))

(event EventBeginPlay
  (Variables|Animation|Swaying|SetInitalMeshRotation (Variables|/Script/Engine.SceneComponent|GetRelativeRotation (Variables|Default|GetStaticMesh)))
  (Variables|Default|SetInitialLocation (Transformation|GetActorLocation)))

(fn ConstructionScript)

(fn UpdateWaterPositition
  (bind _returnvalue (Transformation|GetActorLocation))
  (bind _outhit (Collision|LineTraceByChannel (+ _returnvalue "0, 0,100.000000") (+ _returnvalue "0, 0,-10000.000000") "TraceTypeQuery1" false 0 "None"))
  (Variables|Animation|SetWaterPosition (.ImpactPoint (Collision|BreakHitResult _outhit))))

(fn GetPlayerPositionTransform
  (bind _playerposition (Variables|Default|GetPlayerPosition))
  (bind _returnvalue (Transformation|GetWorldTransform _playerposition))
  (return (Math|Transform|MakeTransform (.location _returnvalue) (.rotation _returnvalue) "1,1,1")))

(fn GetPlayerPositionComponent
  (return (Variables|Default|GetPlayerPosition)))

(fn UpdateBoatLocation
  (params (Delta%20Seconds :type Float%20%28single-precision%29))
  (bind _staticmesh (Variables|Default|GetStaticMesh))
  (bind _relativelocation (Variables|/Script/Engine.SceneComponent|GetRelativeLocation _staticmesh))
  ;[1 1 1] Up Down Animation
  (Transformation|SetRelativeLocation (Variables|Default|GetStaticMesh) (Math|Vector|MakeVector (.x _relativelocation) (.y _relativelocation) (+ (.z _relativelocation) (CallFunction|GetFloatingOffset))) false false)
  ;[1 1 1] ForwardMovement
  (Class|PawnMovementComponent|AddInputVector (Variables|Default|GetFloatingPawnMovement) (Transformation|GetActorForwardVector) false))

(fn GetFloatingOffset
  (return (* (Math|Trig|Sin(Radians) (* (Utilities|Time|GetGameTimeinSeconds) (Variables|Animation|Floating|GetFloatingSpeed))) (Variables|Animation|Floating|GetFloatingHeight))))