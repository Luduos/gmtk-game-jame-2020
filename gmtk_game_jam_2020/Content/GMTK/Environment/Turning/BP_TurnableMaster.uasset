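; BP_TurnableMaster is a turnable environment piece that docks at a target transform and signals when the next piece should spawn.
; MoveToTarget runs a Movement timeline to a dock-offset target, then a Rotation timeline adds RotationAngle to roll.
; A player-controlled pawn touching SpawnNextCollider arms a one-time OnSpawnNextEntered call carrying SpawnNextTarget's transform, held until animation ends.
; BeginPlay also checks existing overlaps, delaying the call so the game mode can bind.
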(event OnComponentBeginOverlap(SpawnNextCollider)
  (params (OverlappedComponent :type Primitive%20Component%20Object%20Reference) (OtherActor :type Actor%20Object%20Reference) (OtherComp :type Primitive%20Component%20Object%20Reference) (OtherBodyIndex :type Integer) (bFromSweep :type Boolean) (SweepResult :type Hit%20Result%20Structure%20%28by%20ref%29))
  ;[1 1 1] Signal that next cube should be spawned
  (CallFunction|UpdateSpawnRequirement OtherActor)
  ;[1 1 1] Try spawn
  (CallFunction|TryCallSpawnNextOnce))

(event Custom|MoveToTarget
  (params (Target :type Transform))
  ;[1 1 1] Movement to target
  (CallFunction|CalcTargetTransform (.location Target) (.rotation Target) (.scale Target))
  (Variables|Animation|Positioning|SetPositioningStart (Transformation|GetActorTransform))
  (bind _normalizedposition (Timeline|Movement PlayFromStart)
    (:Update
      (Transformation|SetActorTransform (Math|Transform|Lerp(Transform) (Variables|Animation|Positioning|GetPositioningStart) (Variables|Animation|Positioning|GetPositioningTarget) _normalizedposition)))
    (:Finished
      (CallFunction|OnMovementFinished))))

(event Custom|TryCallSpawnNextOnce
  ;[1 1 1] Only spawn if touched player and not animating
  (if (Variables|Default|GetbShouldSpawnNext)
    (bind _isanimating (CallFunction|IsAnimating))
    (if (not _isanimating)
      ;[1 1 1] Only spawn once
      (Utilities|FlowControl|DoOnce false
        (:Completed
          (Default|CallOnSpawnNextEntered (Transformation|GetWorldTransform (Variables|Default|GetSpawnNextTarget))))))))

(event Custom|OnMovementFinished
  ;[1 1 1] rotation after reaching target
  (Variables|Default|SetStartingRotation (Transformation|GetActorRotation))
  (bind _rotationnormalized (Timeline|Rotation PlayFromStart)
    (:Update
      (Transformation|SetActorRotation (Math|Rotator|Lerp(Rotator) (Variables|Default|GetStartingRotation) (Math|Rotator|MakeRotator (+ (.roll (Variables|Default|GetStartingRotation)) (Variables|Config|GetRotationAngle)) (.pitch (Variables|Default|GetStartingRotation)) (.yaw (Variables|Default|GetStartingRotation))) _rotationnormalized)))
    (:Finished
      ;[1 1 1] Comment
      (CallFunction|TryCallSpawnNextOnce))))

(event EventBeginPlay
  (bind _spawnnextcollider (Variables|Default|GetSpawnNextCollider))
  ;[1 1 1] Check at the beginning for all overlapping actors, if we're already touching the player
  (bind _outactors (Collision|ComponentOverlapActors _spawnnextcollider (Transformation|GetWorldTransform _spawnnextcollider) (Variables|Default|GetOverlapTargets) "/Script/Engine.Pawn"))
  (bind _array_element (Utilities|Array|ForEachLoopwithBreak _outactors)
    (:LoopBody
      (CallFunction|UpdateSpawnRequirement _array_element)
      ;[1 1 1] Delayed call of on spawn next. Required for the game mode to be able to bind event
      (Utilities|FlowControl|Delay 0.2)
      (CallFunction|TryCallSpawnNextOnce))))

(fn ConstructionScript)

(fn CalcTargetTransform
  (params (PositioningTarget_Location :type Vector) (PositioningTarget_Rotation :type Rotator) (PositioningTarget_Scale :type Vector))
  (Variables|Animation|Positioning|SetPositioningTarget (Math|Transform|MakeTransform (- PositioningTarget_Location (* (Variables|/Script/Engine.SceneComponent|GetRelativeLocation (Variables|Default|GetSpawnDockTarget)) 2)) PositioningTarget_Rotation PositioningTarget_Scale)))

(fn UpdateSpawnRequirement
  (params (OverlappingActor :type Actor%20Object%20Reference))
  (bind _aspawn (Utilities|Casting|CastToPawn OverlappingActor))
  (if (Pawn|IsPlayerControlled _aspawn)
    (Variables|Default|SetbShouldSpawnNext true)))

(fn IsAnimating
  (return (or (Audio|Components|Audio|IsPlaying (Variables|Default|GetRotation)) (Audio|Components|Audio|IsPlaying (Variables|Default|GetMovement)))))