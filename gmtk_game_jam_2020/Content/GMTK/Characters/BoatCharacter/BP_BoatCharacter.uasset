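; BP_BoatCharacter is a character that rides at an assigned position on a boat.
; SetBoatPlayerPosition stores that position and snaps the character onto it, raised by the capsule half-height.
; Each Tick, it copies the position's X, Y and rotation but keeps its own Z, leaving height independent of the boat.
; Damage handling only prints a debug message with the amount.
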(event EventTick
  (params (DeltaSeconds :type Float%20%28single-precision%29))
  (|SyncPlayerPositionToBoat))

(event Game|Damage|EventAnyDamage
  (params (Damage :type Float%20%28single-precision%29) (DamageType :type Damage%20Type%20Object%20Reference) (InstigatedBy :type Controller%20Object%20Reference) (DamageCauser :type Actor%20Object%20Reference))
  (Development|PrintString (Utilities|String|Append (Utilities|String|MakeLiteralString "Autsch! Damage: ") (Utilities|String|ToString(Float) Damage))))

(fn ConstructionScript
  (|CallParentFunction))

(fn SetBoatPlayerPosition
  (params (PlayerPosition :type Scene%20Component%20Object%20Reference))
  (bind _output_get (Variables|Default|SetPositionOnBoat PlayerPosition))
  ;[1 1 1] Set Player Position to boat
  (Transformation|SetActorTransform (Math|Transform|MakeTransform (+ (.location (Transformation|GetWorldTransform _output_get)) (Math|Vector|MakeVector 0.0 0.0 (Variables|/Script/Engine.CapsuleComponent|GetCapsuleHalfHeight (Variables|Default|GetCapsuleComponent)))) (.rotation (Transformation|GetWorldTransform _output_get)) "1,1,1")))